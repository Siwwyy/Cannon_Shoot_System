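; BP_Object_Cannon_Ball is a cannonball projectile actor, scaled down to quarter size by its construction script.
; On BeginPlay it copies its Velocity variable into the ProjectileMovement component.
; When it hits an actor whose display name is "OBSTACLE", it plays a quiet, low-pitched explosion sound at the hit location and destroys itself.
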(event EventBeginPlay
  (Variables|/Script/Engine.MovementComponent|SetVelocity (Variables|Default|GetProjectileMovement) (Variables|Default|GetVelocity)))

(event Collision|EventHit
  (params (MyComp :type Primitive%20Component%20Object%20Reference) (Other :type Actor%20Object%20Reference) (OtherComp :type Primitive%20Component%20Object%20Reference) (bSelfMoved :type Boolean) (HitLocation :type Vector :default "0, 0, 0") (HitNormal :type Vector :default "0, 0, 0") (NormalImpulse :type Vector :default "0, 0, 0") (Hit :type Hit%20Result%20Structure%20%28by%20ref%29))
  (if (Utilities|Enum|Equal(Enum) (Utilities|GetDisplayName Other) "OBSTACLE")
    (Audio|PlaySoundatLocation "/Game/GrenadePack/MapAssets/Audio/Explosion01.Explosion01" HitLocation "0, 0, 0" 0.2 0.5 0.0 0 0 0)
    (Actor|DestroyActor self)))

(fn ConstructionScript
  (Transformation|SetWorldScale3D "0.250000,0.250000,0.250000"))